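; BP_Piece3D is a falling piece for a 3D block board, hard-coded as a straight four-cell line along X.
; On BeginPlay it finds BP_Board3D, anchors near the top centre and starts a looping fall timer.
; TryMove checks the shifted cells with the board's CanPlace, then updates the anchor and calls DrawActive.
; The timer stops when a downward move fails, with no locking or respawn here.
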(event Custom|CustomEvent
  (bind _newparam (CallFunction|TryMove (Utilities|Struct|MakeIntVector 0 0 -1)))
  (if (not _newparam)
    (Utilities|Time|ClearandInvalidateTimerbyHandle (Variables|Default|GetTimer))))

(event EventBeginPlay
  (bind _returnvalue (Actor|GetActorOfClass "/Game/Blueprints/BP_Board3D.BP_Board3D_C"))
  (Variables|Default|SetBoardRef _returnvalue)
  (Utilities|FlowControl|Sequence
    (:then_0
      (Utilities|Array|Add (Variables|Default|GetOffset) (Utilities|Struct|MakeIntVector 0 0))
      (Utilities|Array|Add (Variables|Default|GetOffset) (Utilities|Struct|MakeIntVector 1 0))
      (Utilities|Array|Add (Variables|Default|GetOffset) (Utilities|Struct|MakeIntVector 2 0))
      (Utilities|Array|Add (Variables|Default|GetOffset) (Utilities|Struct|MakeIntVector 3 0)))
    (:then_1
      (Variables|Default|SetAnchor (Utilities|Struct|MakeIntVector (- (/ (Variables|/Game/Blueprints/BP_Board3D.BP_Board3D_C|GetW (Variables|Default|GetBoardRef)) 2) 1) (/ (Variables|/Game/Blueprints/BP_Board3D.BP_Board3D_C|GetD (Variables|Default|GetBoardRef)) 2) (- (Variables|/Game/Blueprints/BP_Board3D.BP_Board3D_C|GetH (Variables|Default|GetBoardRef)) 1)))
      (bind _returnvalue_2 (Utilities|Time|SetTimerbyEvent (delegate Custom|CustomEvent) (Variables|Default|GetFallInterval) true))
      (Variables|Default|SetTimer _returnvalue_2))))

(event EventTick
  (params (DeltaSeconds :type Float%20%28single-precision%29)))

(fn ConstructionScript)

(fn TryMove
  (params (Delta :type Int%20Vector%20Structure))
  (bind _canplace (Default|CanPlace (Variables|Default|GetBoardRef) (Utilities|Struct|MakeIntVector (+ (.x Delta) (.x (Variables|Default|GetAnchor))) (+ (.y Delta) (.y (Variables|Default|GetAnchor))) (+ (.z Delta) (.z (Variables|Default|GetAnchor)))) (Variables|Default|GetOffset)))
  (if _canplace
    (bind _output_get (Variables|Default|SetAnchor (Utilities|Struct|MakeIntVector (+ (.x Delta) (.x (Variables|Default|GetAnchor))) (+ (.y Delta) (.y (Variables|Default|GetAnchor))) (+ (.z Delta) (.z (Variables|Default|GetAnchor))))))
    (Default|DrawActive (Variables|Default|GetBoardRef) _output_get (Variables|Default|GetOffset))
    (return true)
    (else
      (Development|PrintString "Can't Move")
      (return false))))