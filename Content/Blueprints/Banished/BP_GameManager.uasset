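; BP_GameManager runs the piece loop of a 3D falling-block game, spawning pieces and locking them into the board.
; On BeginPlay it finds BP_Board3D, resets score, level and fall speed, then pre-rolls the next random piece type.
; Each spawned BP_Piece3D receives its type and fall interval, and its OnLanded event makes the board lock it and clear layers before the manager destroys it and spawns another.
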(event Custom|SpawnNewPiece
  (Variables|Default|SetThisTypeID (Variables|Default|GetNextTypeID))
  (Variables|Default|SetNextTypeID (Math|Random|RandomInteger 10))
  (bind _returnvalue (Game|SpawnActorfromClass "/Game/Blueprints/BP_Piece3D.BP_Piece3D_C" (Math|Transform|MakeTransform "0, 0, 0" "0, 0, 0" "1.000000,1.000000,1.000000") "Undefined" "MultiplyWithRoot" 0 0))
  (bind _output_get (Variables|Default|SetActivePiece _returnvalue))
  (Variables|/Game/Blueprints/BP_Piece3D.BP_Piece3D_C|SetTypeID _output_get (Variables|Default|GetThisTypeID))
  (Variables|/Game/Blueprints/BP_Piece3D.BP_Piece3D_C|SetFallInterval _output_get (Variables|Default|GetFallInterval))
  (EventDispatchers|BindEventtoOnLanded _output_get (delegate Custom|HandlePieceLanded)))

(event Custom|HandlePieceLanded
  (params (Anchor :type Int%20Vector%20Structure) (Offsets :type Array%20of%20Int%20Vector%20Structures) (TypeID :type Integer))
  (Default|LockPiece (Variables|Default|GetBoardRef) (Variables|/Game/Blueprints/BP_Piece3D.BP_Piece3D_C|GetAnchor (Variables|Default|GetActivePiece)) (Variables|/Game/Blueprints/BP_Piece3D.BP_Piece3D_C|GetOffsets (Variables|Default|GetActivePiece)) (Variables|/Game/Blueprints/BP_Piece3D.BP_Piece3D_C|GetTypeID (Variables|Default|GetActivePiece)))
  (Default|TryClearLayers (Variables|Default|GetBoardRef))
  (Actor|DestroyActor (Variables|Default|GetActivePiece))
  (Variables|Default|SetActivePiece 0)
  (CallFunction|SpawnNewPiece))

(event EventBeginPlay
  (bind _returnvalue (Actor|GetActorOfClass "/Game/Blueprints/BP_Board3D.BP_Board3D_C"))
  (Variables|Default|SetBoardRef _returnvalue)
  (Variables|Default|SetScore 0)
  (Variables|Default|SetLevel 0)
  (Variables|Default|SetTotalCleared 0)
  (Variables|Default|SetFallInterval (Variables|Default|GetBaseFallInterval))
  (Variables|Default|SetNextTypeID (Math|Random|RandomInteger 10))
  (CallFunction|SpawnNewPiece))

(event Collision|EventActorBeginOverlap
  (params (OtherActor :type Actor%20Object%20Reference)))

(event EventTick
  (params (DeltaSeconds :type Float%20%28single-precision%29)))

(fn ConstructionScript)