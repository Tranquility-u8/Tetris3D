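; BP_CameraPawn is the player pawn that handles input for a 3D Tetris game.
; On possession it adds the Tetris Enhanced Input mapping context, and on BeginPlay it caches the GM_Tetris3D actor.
; MoveX and MoveY presses call TryMove on that actor's active piece, stepping it one unit along X or Y by input sign.
; Hard drop, soft drop and rotate input events are empty stubs.
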(event Input|EnhancedActionEvents|EnhancedInputActionIA_MoveX
  (params (ActionValue :type Float%20%28double-precision%29) (ElapsedSeconds :type Float%20%28double-precision%29) (TriggeredSeconds :type Float%20%28double-precision%29) (InputAction :type Input%20Action%20Object%20Reference :default "/Game/Input/IA_MoveX.IA_MoveX"))
  (:Started
    (if (> ActionValue 0.5)
      (Default|TryMove (Variables|/Game/Blueprints/GM_Tetris3D.GM_Tetris3D_C|GetActivePiece (Variables|Default|GetGMRef)) (Utilities|Struct|MakeIntVector 1 0 0))
      (elif (< ActionValue -0.5)
        (Default|TryMove (Variables|/Game/Blueprints/GM_Tetris3D.GM_Tetris3D_C|GetActivePiece (Variables|Default|GetGMRef)) (Utilities|Struct|MakeIntVector -1 0 0))))))

(event Input|EnhancedActionEvents|EnhancedInputActionIA_MoveY
  (params (ActionValue :type Float%20%28double-precision%29) (ElapsedSeconds :type Float%20%28double-precision%29) (TriggeredSeconds :type Float%20%28double-precision%29) (InputAction :type Input%20Action%20Object%20Reference :default "/Game/Input/IA_MoveY.IA_MoveY"))
  (:Started
    (if (> ActionValue 0.5)
      (Default|TryMove (Variables|/Game/Blueprints/GM_Tetris3D.GM_Tetris3D_C|GetActivePiece (Variables|Default|GetGMRef)) (Utilities|Struct|MakeIntVector 0 1 0))
      (elif (< ActionValue -0.5)
        (Default|TryMove (Variables|/Game/Blueprints/GM_Tetris3D.GM_Tetris3D_C|GetActivePiece (Variables|Default|GetGMRef)) (Utilities|Struct|MakeIntVector 0 -1 0))))))

(event Input|EnhancedActionEvents|EnhancedInputActionIA_Rotate
  (params (ActionValue :type Boolean) (ElapsedSeconds :type Float%20%28double-precision%29) (TriggeredSeconds :type Float%20%28double-precision%29) (InputAction :type Input%20Action%20Object%20Reference :default "/Game/Input/IA_Rotate.IA_Rotate")))

(event Input|EnhancedActionEvents|EnhancedInputActionIA_HardDrop
  (params (ActionValue :type Boolean) (ElapsedSeconds :type Float%20%28double-precision%29) (TriggeredSeconds :type Float%20%28double-precision%29) (InputAction :type Input%20Action%20Object%20Reference :default "/Game/Input/IA_HardDrop.IA_HardDrop")))

(event Input|EnhancedActionEvents|EnhancedInputActionIA_SoftDrop
  (params (ActionValue :type Boolean) (ElapsedSeconds :type Float%20%28double-precision%29) (TriggeredSeconds :type Float%20%28double-precision%29) (InputAction :type Input%20Action%20Object%20Reference :default "/Game/Input/IA_SoftDrop.IA_SoftDrop")))

(event EventBeginPlay
  (bind _returnvalue (Actor|GetActorOfClass "/Game/Blueprints/GM_Tetris3D.GM_Tetris3D_C"))
  (Variables|Default|SetGMRef _returnvalue))

(event Collision|EventActorBeginOverlap
  (params (OtherActor :type Actor%20Object%20Reference)))

(event EventTick
  (params (DeltaSeconds :type Float%20%28single-precision%29)))

(event EventPossessed
  (params (NewController :type Controller%20Object%20Reference))
  (bind _asplayer_controller (Utilities|Casting|CastToPlayerController NewController))
  (Input|AddMappingContext (PlayerController|LocalPlayerSubsystems|GetEnhancedInputLocalPlayerSubsystem _asplayer_controller) "/Game/Input/IMC_Tetris.IMC_Tetris" 0 "(bIgnoreAllPressedKeysUntilRelease=True,bForceImmediately=False,bNotifyUserSettings=False)"))

(fn ConstructionScript)