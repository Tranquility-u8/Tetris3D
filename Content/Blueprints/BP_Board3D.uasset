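; BP_Board3D is a 3D grid board actor for placing and previewing multi-cell pieces defined as offsets from an anchor cell.
; Helpers convert cell coordinates to a flattened array index or to world positions scaled by CellSize from the actor's location.
; CanPlace only bounds-checks each cell through IsInside, whose upper limits are inclusive.
; DrawActive rebuilds the ISMActivePreview instances at the piece's cells, printing a debug string for each.
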(event EventBeginPlay)

(event Collision|EventActorBeginOverlap
  (params (OtherActor :type Actor%20Object%20Reference)))

(event EventTick
  (params (DeltaSeconds :type Float%20%28single-precision%29)))

(fn ConstructionScript)

(fn IsInside
  (params (X :type Integer) (Y :type Integer) (Z :type Integer))
  (return (Math|Boolean|ANDBoolean (and (<= X (Variables|Default|GetW)) (>= X 0)) (and (<= Y (Variables|Default|GetD)) (>= Y 0)) (and (<= Z (Variables|Default|GetH)) (>= Z 0)))))

(fn Index
  (params (X :type Integer) (Y :type Integer) (Z :type Integer))
  (return (+ X (* Y (Variables|Default|GetW)) (* Z (Variables|Default|GetW) (Variables|Default|GetD)))))

(fn GridtoWorld
  (params (X :type Integer) (Y :type Integer) (Z :type Integer))
  (return (+ (* (Utilities|Struct|MakeIntVector X Y Z) (Variables|Default|GetCellSize)) (Transformation|GetActorLocation))))

(fn CanPlace
  (params (Anchor :type Int%20Vector%20Structure) (Offset :type Array%20of%20Int%20Vector%20Structures))
  (bind (_x _y _z) (Utilities|Struct|BreakIntVector Anchor))
  (for _array_element Offset
    (if (not (CallFunction|IsInside (+ (.X (Utilities|Struct|BreakIntVector _array_element)) _x) (+ (.Y (Utilities|Struct|BreakIntVector _array_element)) _y) (+ (.Z (Utilities|Struct|BreakIntVector _array_element)) _z)))
      (return false)))
  (return true))

(fn DrawActive
  (params (Anchor :type Int%20Vector%20Structure) (Offset :type Array%20of%20Int%20Vector%20Structures))
  (Components|InstancedStaticMesh|ClearInstances (Variables|Default|GetISM_ActivePreview))
  (for _array_element Offset
    (Components|InstancedStaticMesh|AddInstance (Variables|Default|GetISM_ActivePreview) (Math|Conversions|ToTransform(Vector) (CallFunction|GridtoWorld (+ (.x _array_element) (.x Anchor)) (+ (.y _array_element) (.y Anchor)) (+ (.z _array_element) (.z Anchor)))) true)
    (Development|PrintString "Add Instance")))